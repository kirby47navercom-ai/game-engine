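; BP_FloatingElevator is an elevator actor that rises while something is inside its trigger Box.
; Box overlap begin and end toggle an OnBoard flag, print debug messages, and switch FloatingComponent2 off on entry and back on at exit.
; While OnBoard is set, Tick moves the actor up by a fixed local Z offset each frame, unscaled by delta time and without sweep.
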(event OnComponentBeginOverlap(Box)
  (params (OverlappedComponent :type Primitive%20Component%20Object%20Reference) (OtherActor :type Actor%20Object%20Reference) (OtherComp :type Primitive%20Component%20Object%20Reference) (OtherBodyIndex :type Integer) (bFromSweep :type Boolean) (SweepResult :type Hit%20Result%20Structure%20%28by%20ref%29))
  (Development|PrintString "On Board")
  (Variables|Default|SetOn%20Board? true)
  (Default|TurnOff (Variables|Default|GetFloatingComponent2)))

(event OnComponentEndOverlap(Box)
  (params (OverlappedComponent :type Primitive%20Component%20Object%20Reference) (OtherActor :type Actor%20Object%20Reference) (OtherComp :type Primitive%20Component%20Object%20Reference) (OtherBodyIndex :type Integer))
  (Development|PrintString "Off Board")
  (Variables|Default|SetOn%20Board? false)
  (Default|Turnon (Variables|Default|GetFloatingComponent2)))

(event EventBeginPlay)

(event Collision|EventActorBeginOverlap
  (params (OtherActor :type Actor%20Object%20Reference)))

(event EventTick
  (params (DeltaSeconds :type Float%20%28single-precision%29))
  (if (Variables|Default|GetOn%20Board?)
    (Transformation|AddActorLocalOffset "0.000000,0.000000,1.000000" false false)))

(fn ConstructionScript)