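; BP_AutoFence is a procedural fence actor that builds a row of static meshes from its origin to the FenceEnd vector.
; The Construction Script normalizes FenceEnd into a direction and adds a mesh component every 20 units along it, rotated to face that direction.
; Each piece gets a tiny random Z-scale jitter.
; The Event Graph holds only disabled placeholder events, so there is no runtime logic.
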(event EventBeginPlay)

(event Collision|EventActorBeginOverlap
  (params (OtherActor :type Actor%20Object%20Reference)))

(event EventTick
  (params (DeltaSeconds :type Float%20%28single-precision%29)))

(fn ConstructionScript
  (bind _fenceend (Variables|Default|GetFenceEnd))
  (Variables|Default|Set단위방향벡터 (Math|Vector|Normalize _fenceend))
  (for _index (range 0 (/ (Math|Vector|VectorLength _fenceend) 2e+01))
    (AddComponent|AddStaticMeshComponent false (Math|Transform|MakeTransform (* _index 2e+01 (Variables|Default|Get단위방향벡터)) (Math|Conversions|RotationFromXVector (Variables|Default|Get단위방향벡터)) (Math|Vector|MakeVector 1.0 1.0 (Math|Random|RandomFloatinRange 0.999 1.001))))))